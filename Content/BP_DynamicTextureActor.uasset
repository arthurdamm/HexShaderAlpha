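; Test actor that draws colored rectangles through its TextureActorComponent in response to key presses.
; The construction script creates a dynamic instance of M_DynamicMaterial on the Plane, stores it, and hands it to the component.
; BeginPlay enables input from the first player controller, so the O and P keys each call DrawRectangle with the same size but a different color.
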(event `self.ReceiveBeginPlay`
  (`self.EnableInput` (`GameplayStatics.GetPlayerController` 0)))

(event `Key|O`
  (params (Key :type "Key Structure"))
  (:`Pressed`
    (`TextureActorComponent.DrawRectangle` (`self.TextureActorComponent`) 0 0 50 50 (struct :`R` 0.175016 :`G` 0.054074 :`B` 1.0 :`A` 1.0))))

(event `Key|P`
  (params (Key :type "Key Structure"))
  (:`Pressed`
    (`TextureActorComponent.DrawRectangle` (`self.TextureActorComponent`) 0 0 50 50 (struct :`R` 0.419724 :`G` 1.0 :`B` 0.263633 :`A` 1.0))))

(fn `UserConstructionScript`
  (bind _returnvalue (`PrimitiveComponent.CreateDynamicMaterialInstance` (`self.Plane`) 0 "/Game/M_DynamicMaterial.M_DynamicMaterial" "None"))
  (bind _output_get (set `self.Dynamic Material Var` _returnvalue))
  (set `TextureActorComponent.DynamicMaterial` _output_get (`self.TextureActorComponent`)))