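; BP_ColorChangeObject is a test actor that recolors the materials on its Cube mesh at runtime.
; On BeginPlay it creates a dynamic material instance for each material slot and stores them in an array.
; SetMyValues then pushes the Color, Roughness and Metallic parameters from the actor's variables to every stored instance.
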(event `self.ReceiveBeginPlay`
  (bind _cube (`self.Cube`))
  (for (_array_element _array_index) (`MeshComponent.GetMaterials` _cube)
    (bind _returnvalue (`PrimitiveComponent.CreateDynamicMaterialInstance` _cube _array_index _array_element "None"))
    (`KismetArrayLibrary.Array_Set` (`self.DynamicMaterialInstances`) _array_index _returnvalue true))
  (`self.SetMyValues`))

(event `SetMyValues`
  (for _array_element (`self.DynamicMaterialInstances`)
    (`MaterialInstanceDynamic.SetVectorParameterValue` _array_element "Color" (`self.Value`))
    (`MaterialInstanceDynamic.SetScalarParameterValue` _array_element "Roughness" (`self.Value_0`))
    (`MaterialInstanceDynamic.SetScalarParameterValue` _array_element "Metallic" (`self.Value_1`))))

(fn `UserConstructionScript`)